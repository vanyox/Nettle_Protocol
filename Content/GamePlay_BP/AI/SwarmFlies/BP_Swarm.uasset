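; Fly swarm enemy that chases the GG-tagged character and deals repeating damage while it overlaps the inner damage sphere.
; The outer sphere starts tick-driven AI moves without pathfinding and feeds the target to the Niagara effect, while a looping timer checks when to stop.
; Weapon hits wear down its hit count and fire weapons kill it instantly, fading the effect before destruction.
; The construction script adjusts its height from a line trace.
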(event `self.ReceiveBeginPlay`
  (set `self.InitLocation` (`self.K2_GetActorLocation`)))

(event `self.DamageSphere.OnComponentBeginOverlap`
  (params (OverlappedComponent :type "PrimitiveComponent Object Reference") (OtherActor :type "Actor Object Reference") (OtherComp :type "PrimitiveComponent Object Reference") (OtherBodyIndex :type Integer) (bFromSweep :type Boolean) (SweepResult :type "HitResult Structure (by ref)"))
  (if (`self.ActorHasTag` OtherActor "GG")
    (if (`ActorComponent.ComponentHasTag` OtherComp "Weapon")
      (if (`ActorComponent.ComponentHasTag` OtherComp "Fire")
        (set `self.HpHit` 0)
        (else
          (`/Engine/EditorBlueprintResources/StandardMacros.DecrementInt` (`self.HpHit`)
            (:`  `
              _))))
      (if (<= (`self.HpHit`) 0)
        (`ActorComponent.Deactivate` (`self.NS_SwarmFlies`))
        (`PrimitiveComponent.SetCollisionEnabled` (`self.DamageSphere`) "NoCollision")
        (`PrimitiveComponent.SetCollisionEnabled` (`self.ActiveSphere`) "NoCollision")
        (`KismetSystemLibrary.Delay` 2.0)
        (`self.K2_DestroyActor`))
      (elif (not (`KismetSystemLibrary.K2_IsTimerActive` null "Damage"))
        (`self.Damage`)))))

(event `self.ActiveSphere.OnComponentBeginOverlap`
  (params (OverlappedComponent :type "PrimitiveComponent Object Reference") (OtherActor :type "Actor Object Reference") (OtherComp :type "PrimitiveComponent Object Reference") (OtherBodyIndex :type Integer) (bFromSweep :type Boolean) (SweepResult :type "HitResult Structure (by ref)"))
  (if (`self.ActorHasTag` OtherActor "GG")
    (set `self.OverlapActor` OtherActor)
    (`FXSystemComponent.SetBoolParameter` (`self.NS_SwarmFlies`) "FindTarget" true)
    (`KismetSystemLibrary.K2_SetTimer` null "HasOverlapGG" 5.0 true)
    (`self.SetActorTickEnabled` true)
    (`self.SetTargetLocationTarget`)
    (`self.MoveToGG`)))

(event `self.ActiveSphere.OnComponentEndOverlap`
  (params (OverlappedComponent :type "PrimitiveComponent Object Reference") (OtherActor :type "Actor Object Reference") (OtherComp :type "PrimitiveComponent Object Reference") (OtherBodyIndex :type Integer))
  (`self.SetTargetLocationTarget`)
  (`self.MoveToGG`))

(event `self.ReceiveTick`
  (params (DeltaSeconds :type "Float (single-precision)"))
  (`self.SetTargetLocationTarget`)
  (`self.MoveToGG`))

(event `MoveToGG`
  (bind _returnvalue (`AIBlueprintHelperLibrary.GetAIController` self))
  (`/Engine/EditorBlueprintResources/StandardMacros.IsValid` _returnvalue
    (:`Is Valid`
      (`AIController.MoveToLocation` _returnvalue (`self.TargetLocation`) 1.0 false false false true null true))))

(fn `Damage`
  (if (`PrimitiveComponent.IsOverlappingActor` (`self.DamageSphere`) (`self.OverlapActor`))
    (message `/Game/GamePlay_BP/Interface/BPI_Damage.Damage` (`self.OverlapActor`) self 2.0 (0.0 0.0 0.0))
    (`KismetSystemLibrary.K2_SetTimer` null "Damage" 1.0)))

(fn `HasOverlapGG`
  (locals (OverlapGG :type Boolean))
  (for _array_element (`PrimitiveComponent.GetOverlappingActors` (`self.ActiveSphere`) "/Script/Engine.Character")
    (if (`self.ActorHasTag` _array_element "GG")
      (set `local.OverlapGG` true)
      (break)))
  (if (not (`local.OverlapGG`))
    (`KismetSystemLibrary.K2_ClearTimer` null "HasOverlapGG")
    (set `self.OverlapActor` null)
    (`self.SetActorTickEnabled` false)
    (`MovementComponent.StopMovementImmediately` (`self.FloatingPawnMovement`))
    (`FXSystemComponent.SetBoolParameter` (`self.NS_SwarmFlies`) "FindTarget" false)))

(fn `SetTargetLocationTarget`
  (bind _overlapactor (`self.OverlapActor`)
    (:`then`
      (set `self.TargetLocation` (`self.K2_GetActorLocation` _overlapactor))
      (`NiagaraComponent.SetVariablePosition` (`self.NS_SwarmFlies`) "Target" (`self.TargetLocation`)))
    (:`else`)))

(fn `UserConstructionScript`
  (locals (UpVector :type "Float (single-precision)" :default -150.0))
  (bind (_returnvalue_x _returnvalue_y) (`KismetMathLibrary.BreakVector` (`self.K2_GetActorLocation`)))
  (bind _returnvalue (`self.K2_GetActorLocation`))
  (bind (_outhit _returnvalue_2) (`KismetSystemLibrary.LineTraceSingle` :`Start` _returnvalue :`End` (+ _returnvalue (* (`self.GetActorUpVector`) (`local.UpVector`))) :`TraceChannel` "TraceTypeQuery1" :`DrawDebugType` "ForDuration"))
  (if _returnvalue_2
    (bind (_bblockinghit _binitialoverlap _time _distance _location _impactpoint _normal _impactnormal _physmat _hitactor _hitcomponent _hitbonename _bonename _hititem _elementindex _faceindex _tracestart _traceend) (`GameplayStatics.BreakHitResult` _outhit))
    (bind (_returnvalue_x_2 _returnvalue_y_2 _returnvalue_z) (`KismetMathLibrary.BreakVector` (+ (- _location _traceend) (* (`self.GetActorUpVector`) (`KismetMathLibrary.Abs` (`local.UpVector`))))))
    (`self.K2_SetActorLocation` (`KismetMathLibrary.MakeVector` _returnvalue_x _returnvalue_y _returnvalue_z))))