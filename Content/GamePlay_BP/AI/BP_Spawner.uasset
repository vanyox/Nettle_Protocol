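; Wave spawner for a survival mode that spawns BP_LiveNettle AI until the level's quota N is reached.
; StartBattle enables Tick, which counts down a randomized delay and runs an EQS query around the player.
; A random result location gets an AI facing the player, with debug spheres drawn and the HUD updated.
; Destroyed pawns count toward showing the finish widget, and ResetAndUpdateLevel multiplies the quota by the new level.
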(event `self.ReceiveBeginPlay`
  (bind _output_get (set `self.Player` (`GameplayStatics.GetPlayerPawn` 0)))
  (`/Engine/EditorBlueprintResources/StandardMacros.IsValid` _output_get
    (:`Is Valid`
      (bind _asb_hud (cast `/Game/GamePlay_BP/Base/B_HUD` (`PlayerController.GetHUD` (`GameplayStatics.GetPlayerController` 0))))
      (bind _output_get_2 (set `self.HUD` _asb_hud))
      (add `/Game/UI/Hud/W_Hud.StartGame` (`/Game/GamePlay_BP/Base/B_HUD.GetWidget` (`self.HUD`)) (`|CreateDelegate` :!event `StartBattle`))
      (bind _widget (message `/Game/GamePlay_BP/Interface/BPI_Hud.GetWidgetHud` (`self.HUD`)))
      (`/Game/UI/Hud/W_Hud.ChecketLastNettleBar` _widget (`self.N`)))))

(event `self.ReceiveTick`
  (params (DeltaSeconds :type "Float (single-precision)"))
  (bind _delayspawn (`self.DelaySpawn`))
  (bind _output_get (set `self.LocalTime` (`self.CalculateTIme` DeltaSeconds)))
  (if (== _output_get 0.0)
    (`self.Is Spawn`
      (:`true`
        (`self.Eqs`
          (:`then`)
          (:`else`
            (`self.RunEqs`)
            (set `self.LocalTime` (`KismetMathLibrary.RandomFloatInRange` (- _delayspawn 0.5) (+ _delayspawn 0.5)))))))))

(event `StartBattle`
  (`self.SetActorTickEnabled` true)
  (`self.Is Spawn`
    (:`true`
      (`self.RunEqs`))))

(fn `DestroyPawn`
  (params (DestroyedActor :type "Actor Object Reference"))
  (`/Engine/EditorBlueprintResources/StandardMacros.IncrementInt` (`self.KillNpc`)
    (:`  `
      (if (<= (`self.N`) (`self.KillNpc`))
        (bind _returnvalue (`|CreateWidget` "/Game/GamePlay_BP/Interacts/Bust/Ui/W_IsFinishSurvivel.W_IsFinishSurvivel_C" null (`self.Level`) self))
        (`UserWidget.AddToViewport` _returnvalue 1)))))

(fn `ResetAndUpdateLevel`
  (`/Engine/EditorBlueprintResources/StandardMacros.IncrementInt` (`self.Level`)
    (:`  `
      (set `self.N` (* (`self.N`) (`self.Level`)))
      (`KismetArrayLibrary.Array_Clear` (`self.AllNPC`))
      (set `self.KillNpc` 0)
      (bind _widget (message `/Game/GamePlay_BP/Interface/BPI_Hud.GetWidgetHud` (`self.HUD`)))
      (`/Game/UI/Hud/W_Hud.ChecketLastNettleBar` _widget (`self.N`)))))

(fn `ReturnEQS`
  (params (QueryInstance :type "EnvQueryInstanceBlueprintWrapper Object Reference") (QueryStatus :type "EEnvQueryStatus Enum" :default "Processing"))
  (locals (L_SpawnLocation :type "Vector Structure"))
  (switch `EEnvQueryStatus` QueryStatus
    (:`Processing`
      (set `self.Eqs` null :!label _label))
    (:`Success`
      (bind _resultlocations (`EnvQueryInstanceBlueprintWrapper.GetQueryResultsAsLocations` QueryInstance :!label _label_2))
      (`|ExecutionSequence`
        (:`then_0`
          (for _array_element _resultlocations
            (`KismetSystemLibrary.DrawDebugSphere` _array_element 25.0 12 (struct :`R` 1.0 :`G` 1.0 :`A` 1.0) 1.0 1.0)))
        (:`then_1`
          (set `local.L_SpawnLocation` (`KismetArrayLibrary.Array_Random` _resultlocations))
          (bind _returnvalue (`AIBlueprintHelperLibrary.SpawnAIFromClass` "/Game/GamePlay_BP/AI/BP_LiveNettle.BP_LiveNettle_C" null (`local.L_SpawnLocation`) (`KismetMathLibrary.FindLookAtRotation` (`local.L_SpawnLocation`) (`self.K2_GetActorLocation` (`self.Player`))) false null))
          (add `self.OnDestroyed` _returnvalue (`|CreateDelegate` :!event `DestroyPawn`))
          (`KismetArrayLibrary.Array_Add` (`self.AllNPC`) _returnvalue)
          (set `self.Eqs` null)
          (`KismetSystemLibrary.DrawDebugSphere` (`local.L_SpawnLocation`) 30.0 12 (struct :`G` 1.0 :`A` 1.0) 1.0 1.0)
          (`/Game/GamePlay_BP/Base/B_HUD.UpdateInfoNettle` (`self.HUD`) (`self.AllNPC`)))))
    (:`Failed`
      (goto _label))
    (:`Aborted`
      (goto _label_2))
    (:`OwnerLost`
      (goto _label))
    (:`MissingParam`
      (goto _label))))

(fn `RunEqs`
  (bind _returnvalue (`EnvQueryManager.RunEQSQuery` "/Game/GamePlay_BP/AI/Eqs/BEQ_SpawnNpc.BEQ_SpawnNpc" (`self.Player`) "AllMatching"))
  (bind _output_get (set `self.Eqs` _returnvalue))
  (add `EnvQueryInstanceBlueprintWrapper.OnQueryFinishedEvent` _output_get (`|CreateDelegate` :!event `ReturnEQS`)))

(fn `UserConstructionScript`)