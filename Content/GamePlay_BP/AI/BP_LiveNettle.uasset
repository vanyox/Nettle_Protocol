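; BP_LiveNettle is a living nettle character that is destroyed when a component tagged Weapon overlaps its capsule.
; On destruction it spawns a Niagara burst, passing its own static mesh as a user variable before activation, then randomly may spawn a B_Bust of random type.
; SetDaze temporarily cuts walk speed by a fixed amount, and a named timer calls RemoveDaze to restore the saved speed.
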(event `self.CapsuleComponent.OnComponentBeginOverlap`
  (params (OverlappedComponent :type "PrimitiveComponent Object Reference") (OtherActor :type "Actor Object Reference") (OtherComp :type "PrimitiveComponent Object Reference") (OtherBodyIndex :type Integer) (bFromSweep :type Boolean) (SweepResult :type "HitResult Structure (by ref)"))
  (if (`ActorComponent.ComponentHasTag` OtherComp "Weapon")
    (`self.K2_DestroyActor`)))

(event `self.ReceiveDestroyed`
  (`|ExecutionSequence`
    (:`then_0`
      (bind _returnvalue (`NiagaraFunctionLibrary.SpawnSystemAtLocation` "/Game/GamePlay_BP/Particle/NettleDestruct/NS_DestructNettle.NS_DestructNettle" (`SceneComponent.K2_GetComponentLocation` (`self.StaticMesh`)) (`self.K2_GetActorRotation`) (1.0 1.0 1.0) true false))
      (`NiagaraFunctionLibrary.OverrideSystemUserVariableStaticMesh` _returnvalue "STM" (`StaticMeshComponent.StaticMesh` (`self.StaticMesh`)))
      (`ActorComponent.SetActive` _returnvalue true false))
    (:`then_1`
      (if (`KismetMathLibrary.RandomBoolWithWeight` 0.5)
        (`|SpawnActorFromClass` "/Game/GamePlay_BP/Interacts/Bust/B_Bust.B_Bust_C" (`KismetMathLibrary.MakeTransform` (`SceneComponent.K2_GetComponentLocation` (`self.StaticMesh`)) (struct :`Yaw` 180.0)) "Undefined" "MultiplyWithRoot" null (cast `/Game/GamePlay_BP/Interacts/Bust/Data/E_TypeBust` (`KismetMathLibrary.Conv_IntToByte` (`KismetMathLibrary.RandomIntegerInRange` 0 7))) null)))))

(fn `RemoveDaze`
  (set `CharacterMovementComponent.MaxWalkSpeed` (`self.Max Walk Speed`) (`self.CharacterMovement`)))

(fn `SetDaze`
  (params (TimeActive :type "Float (double-precision)"))
  (returns (Return :type Boolean))
  (`KismetSystemLibrary.K2_SetTimer` null "RemoveDaze" TimeActive)
  (set `self.Max Walk Speed` (`CharacterMovementComponent.MaxWalkSpeed` (`self.CharacterMovement`)))
  (set `CharacterMovementComponent.MaxWalkSpeed` (- (`self.Max Walk Speed`) 400.0) (`self.CharacterMovement`))
  (return false))

(fn `UserConstructionScript`)