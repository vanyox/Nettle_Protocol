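; Campfire actor with a radius-driven Niagara fire, a looping-style fire sound and a dynamic wood material.
; The construction script applies radius, particle rate and initial active state.
; ActiveFire toggles effects and sound, playing the Spawn timeline meant to ramp particle rate and material temperature.
; RegenerateCampfire scatters randomly tilted, center-facing instanced logs around the radius; damage, auto-toggle and grid-spawning logic are left unwired.
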(event `self.ReceiveBeginPlay`)

(fn `ActiveFire`
  (params (Active :type Boolean))
  (bind _output_get (set `self.B_ActiveFire` Active))
  (if _output_get
    (`ActorComponent.Activate` (`self.NS_Fire`) false)
    (`TimelineComponent.PlayFromStart` (`self.Spawn`))
    (`AudioComponent.Play` (`self.MS_RandomStereo_Fire`) 0.0)
    (else
      (`ActorComponent.Deactivate` (`self.NS_Fire`))
      (`AudioComponent.Stop` (`self.MS_RandomStereo_Fire`)))))

(fn `RegenerateCampfire`
  (locals (L_Location :type "Vector Structure" :default (0.0 0.0 0.0)) (L_YRot :type "Float (double-precision)" :default 0.0) (L_ScaleX :type "Float (double-precision)"))
  (bind _l_scalex (`local.L_ScaleX`))
  (bind (_returnvalue_roll _returnvalue_pitch _returnvalue_yaw) (`KismetMathLibrary.BreakRotator` (`KismetMathLibrary.FindLookAtRotation` (`local.L_Location`) (`KismetMathLibrary.MakeVector` 0.0))))
  (bind _returnvalue (/ _l_scalex 1.2))
  (bind _sphereradius (`SphereComponent.SphereRadius` (`self.Sphere`)))
  (`InstancedStaticMeshComponent.ClearInstances` (`self.HierarchicalInstancedStaticMesh`))
  (for _ (range (+ (`self.Last Index`) 1))
    (set `local.L_Location` (* (`KismetMathLibrary.GreaterGreater_VectorRotator` (`self.GetActorRightVector`) (`KismetMathLibrary.MakeRotator` 0.0 0.0 (`KismetMathLibrary.RandomFloatInRange` -180.0 180.0))) (`KismetMathLibrary.RandomFloatInRange` (+ _sphereradius 10.0) (- _sphereradius 10.0))))
    (set `local.L_YRot` (`KismetMathLibrary.RandomFloatInRange` 25.0 45.0))
    (set `local.L_ScaleX` (/ (+ (`SphereComponent.SphereRadius` (`self.Sphere`)) (`local.L_YRot`)) 72.0))
    (`InstancedStaticMeshComponent.AddInstance` (`self.HierarchicalInstancedStaticMesh`) (`KismetMathLibrary.MakeTransform` (`local.L_Location`) (`KismetMathLibrary.MakeRotator` (`KismetMathLibrary.RandomFloatInRange` -180.0 180.0) (`local.L_YRot`) _returnvalue_yaw) (`KismetMathLibrary.MakeVector` _l_scalex _returnvalue _returnvalue)) false)))

(fn `SpawnInstance`
  (locals (L_LastIndex_X :type Integer) (L_LastIndex_Y :type Integer) (L_X_Location :type "Float (double-precision)" :default 0.0) (L_Y_Location :type "Float (double-precision)" :default 0.0)))

(fn `UserConstructionScript`
  (`self.SetActorScale3D` (1.0 1.0 1.0))
  (`SphereComponent.SetSphereRadius` (`self.Sphere`) (`self.RadiusCollision`) true)
  (`FXSystemComponent.SetFloatParameter` (`self.NS_Fire`) "RadiuseSpawn" (- (`self.RadiusCollision`) 30.0))
  (`FXSystemComponent.SetFloatParameter` (`self.NS_Fire`) "SpawnRate" (`self.ParticleSpawn`))
  (`ActorComponent.SetAutoActivate` (`self.NS_Fire`) (`self.B_ActiveFire`))
  (`ActorComponent.SetAutoActivate` (`self.MS_RandomStereo_Fire`) (`self.B_ActiveFire`))
  (`self.DynMat`
    (:`then`)
    (:`else`
      (bind _returnvalue (`PrimitiveComponent.CreateDynamicMaterialInstance` (`self.HierarchicalInstancedStaticMesh`) 0 "/Game/Megascans/3D_Assets/Old_Wood_Boards_ricaS/MI_Old_Wood_Boards_ricaS_2K.MI_Old_Wood_Boards_ricaS_2K" "None"))
      (set `self.DynMat` _returnvalue))))