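; Interact actor that acts as a completion gate, playing its level sequences once every entry in its CheckFInish list has been cleared.
; The construction script resets scale to one and binds an event to each entry's SequencePlay dispatcher.
; CheckPlay removes the given entry and plays all sequences when the list empties.
; BindOverlap binds begin-overlap on child box, sphere and capsule components, but its construction-script call is disconnected.
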(fn `CheckPlay`
  (params (Init :type "/Game/GamePlay_BP/Interacts/BP_Hit Object Reference"))
  (`KismetArrayLibrary.Array_RemoveItem` (`self.CheckFInish`) Init)
  (if (== (`KismetArrayLibrary.Array_Length` (`self.CheckFInish`)) 0)
    (for (_ _array_index) (`self.Level_Sequence`)
      (`self.PlaySeq` _array_index))))

(fn `UserConstructionScript`
  (`parent.UserConstructionScript`)
  (`self.SetActorScale3D` (1.0 1.0 1.0))
  (for _array_element (`self.CheckFInish`)
    (add `/Game/GamePlay_BP/Interacts/BP_Hit.SequencePlay` _array_element (`|CreateDelegate` :!event `CheckPlay`))))