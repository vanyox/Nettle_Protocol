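; BP_SeqInteract is an interactable actor that starts level sequences when used.
; Overlapping its StartInteractCube turns the other actor's trace interact message on, and leaving turns it off.
; Interact sets BlockOverlap and plays every entry in the LevelSequence array, and CanInteract then returns false, making it single-use.
; The construction script forces actor scale to one after running the parent's.
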(event `self.StartInteractCube.OnComponentBeginOverlap`
  (params (OverlappedComponent :type "PrimitiveComponent Object Reference") (OtherActor :type "Actor Object Reference") (OtherComp :type "PrimitiveComponent Object Reference") (OtherBodyIndex :type Integer) (bFromSweep :type Boolean) (SweepResult :type "HitResult Structure (by ref)"))
  (message `/Game/GamePlay_BP/Interface/BPI_CharSetting.UpdateTraceInteract` OtherActor true))

(event `self.StartInteractCube.OnComponentEndOverlap`
  (params (OverlappedComponent :type "PrimitiveComponent Object Reference") (OtherActor :type "Actor Object Reference") (OtherComp :type "PrimitiveComponent Object Reference") (OtherBodyIndex :type Integer))
  (message `/Game/GamePlay_BP/Interface/BPI_CharSetting.UpdateTraceInteract` OtherActor false))

(fn `CanInteract`
  (returns (Return :type Boolean))
  (return (not (`self.BlockOverlap`))))

(fn `Interact`
  (returns (Return :type Boolean))
  (set `self.BlockOverlap` true)
  (for (_ _array_index) (`self.Level_Sequence`)
    (`self.PlaySeq` _array_index))
  (return true))

(fn `UserConstructionScript`
  (`parent.UserConstructionScript`)
  (`self.SetActorScale3D` (1.0 1.0 1.0)))