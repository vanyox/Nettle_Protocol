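; BP_Hit is an interactable actor that plays level sequences after being struck by a weapon a set number of times.
; A Sphere overlap with a component tagged "Weapon" decrements the NHit counter.
; When the counter reaches zero, BlockOverlap latches to ignore further hits and every entry in the LevelSequence array is played.
; The construction script forces the actor's scale to one.
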(event `self.Sphere.OnComponentBeginOverlap`
  (params (OverlappedComponent :type "PrimitiveComponent Object Reference") (OtherActor :type "Actor Object Reference") (OtherComp :type "PrimitiveComponent Object Reference") (OtherBodyIndex :type Integer) (bFromSweep :type Boolean) (SweepResult :type "HitResult Structure (by ref)"))
  (if (`ActorComponent.ComponentHasTag` OtherComp "Weapon")
    (if (not (`self.BlockOverlap`))
      (bind _result (`/Engine/EditorBlueprintResources/StandardMacros.DecrementInt` (`self.N_Hit`))
        (:`  `
          (if (<= _result 0)
            (set `self.BlockOverlap` true)
            (for (_ _array_index) (`self.Level_Sequence`)
              (`self.PlaySeq` _array_index))))))))

(fn `UserConstructionScript`
  (`parent.UserConstructionScript`)
  (`self.SetActorScale3D` (1.0 1.0 1.0)))