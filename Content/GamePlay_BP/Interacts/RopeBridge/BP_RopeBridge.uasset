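; Procedural physics rope bridge that builds itself in the construction script from a plank count, with a stretched cube as a debug preview.
; Planks are chained by physics constraints with both ends fixed, alongside spline mesh ropes and instanced posts, railing ropes and windings.
; Plank rope spline meshes follow the moving planks every tick while a "GG"-tagged actor is inside the generated capsule.
; On BeginPlay and overlap exit, a short looping timer updates them instead.
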(event `EnableTimer`
  (`KismetSystemLibrary.K2_SetTimer` null "DynamicUpdateSpline" 0.1 true)
  (`KismetSystemLibrary.Delay` 3.0)
  (`KismetSystemLibrary.K2_ClearTimer` null "DynamicUpdateSpline"))

(event `self.ReceiveBeginPlay`
  (`self.EnableTimer`))

(event `self.ReceiveTick`
  (params (DeltaSeconds :type "Float (single-precision)"))
  (`self.DynamicUpdateSpline`))

(fn `AddInstanceSTM`
  (locals (L_Scale :type "Vector Structure" :default (0.5 0.5 0.7)) (L_InstanceCom :type "HierarchicalInstancedStaticMeshComponent Object Reference"))
  (bind _returnvalue (`KismetMathLibrary.RandomFloatInRange` 0.0 5.0))
  (bind _returnvalue_2 (`KismetMathLibrary.RandomFloatInRange` 10.0 15.0))
  (bind _l_scale (`local.L_Scale`))
  (bind _returnvalue_3 (`KismetMathLibrary.Conv_IntToDouble` (* (`self.Len`) 25)))
  (`|ExecutionSequence`
    (:`then_0`
      (bind _returnvalue_4 (`AddComponent|NODE_AddHierarchicalInstancedStaticMeshComponent-0`))
      (bind _output_get (set `local.L_InstanceCom` _returnvalue_4))
      (for _index (range 4)
        (`InstancedStaticMeshComponent.AddInstance` _output_get (select `int` _index :`0` (`KismetMathLibrary.MakeTransform` (0.0 85.0 -25.0) (`KismetMathLibrary.MakeRotator` _returnvalue _returnvalue_2 -90.0) _l_scale) :`1` (`KismetMathLibrary.MakeTransform` (0.0 -85.0 -25.0) (`KismetMathLibrary.MakeRotator` _returnvalue _returnvalue_2 90.0) _l_scale) :`2` (`KismetMathLibrary.MakeTransform` (`KismetMathLibrary.MakeVector` _returnvalue_3 85.0 -25.0) (`KismetMathLibrary.MakeRotator` _returnvalue _returnvalue_2 -90.0) _l_scale) :`3` (`KismetMathLibrary.MakeTransform` (`KismetMathLibrary.MakeVector` _returnvalue_3 -85.0 -25.0) (`KismetMathLibrary.MakeRotator` _returnvalue _returnvalue_2 90.0) _l_scale)) false)))
    (:`then_1`
      (for _index_2 (range 3)
        (`self.GenerateSplineAtInstSTM` (`local.L_InstanceCom`) (select `int` _index_2 :`0` 100 :`1` 150 :`2` 200))))
    (:`then_2`
      (`self.GenerateInstStmRopeWinding` (`local.L_InstanceCom`) (`|MakeArray` 100 150 200)))
    (:`then_3`
      (bind _returnvalue_5 (`AddComponent|NODE_AddHierarchicalInstancedStaticMeshComponent-3`))
      (`|ExecutionSequence`
        (:`then_0`
          _)
        (:`then_1`
          _))
      (bind _isa (`/Engine/EditorBlueprintResources/StandardMacros.FlipFlop`)
        (:`A`
          _)
        (:`B`
          _))
      (`InstancedStaticMeshComponent.AddInstance` _returnvalue_5 (`KismetMathLibrary.MakeTransform` (`KismetMathLibrary.MakeVector` (select `bool` _isa :`false` (`KismetMathLibrary.Conv_IntToDouble` (+ (* (+ (`self.Len`) 1) 25) 5)) :`true` -28.0) 0.0 -5.0) (`KismetMathLibrary.MakeRotator` (select `bool` _isa :`false` 15.0 :`true` -15.0) 180.0 90.0) (1.0 1.5 1.0)) false))))

(fn `BeginOverlap`
  (params (OverlappedComponent :type "PrimitiveComponent Object Reference") (OtherActor :type "Actor Object Reference") (OtherComp :type "PrimitiveComponent Object Reference") (OtherBodyIndex :type Integer) (bFromSweep :type Boolean) (SweepResult :type "HitResult Structure (by ref)"))
  (if (`self.ActorHasTag` OtherActor "GG")
    (`self.SetActorTickEnabled` true)
    (return)))

(fn `DynamicUpdateSpline`
  (locals (L_EvenNumber :type Boolean) (L_SelectIndexElement :type "SplineMeshComponent Object Reference"))
  (bind _l_selectindexelement (`local.L_SelectIndexElement`))
  (bind _returnvalue_x (`KismetMathLibrary.BreakVector` (`SplineMeshComponent.GetStartPosition` _l_selectindexelement)))
  (bind _returnvalue_x_2 (`KismetMathLibrary.BreakVector` (`SplineMeshComponent.GetEndPosition` _l_selectindexelement)))
  (bind _relativelocation (`SceneComponent.RelativeLocation` (`local.L_SelectIndexElement`)))
  (bind _keys (`BlueprintMapLibrary.Map_Keys` (`self.NewVar`)))
  (for (_array_element _array_index) _keys
    (set `local.L_SelectIndexElement` _array_element)
    (set `local.L_EvenNumber` (> (mod _array_index 2) 0))
    (bind _values (`BlueprintMapLibrary.Map_Values` (`self.NewVar`)))
    (bind (_output_1 _output_2) (break `/Game/GamePlay_BP/Interacts/RopeBridge/BST_MeshAtSpline` (`|GetArrayItem` _values _array_index)))
    (bind (_returnvalue_x_3 _returnvalue_y _returnvalue_z) (`KismetMathLibrary.BreakVector` (- (`self.GetLocalLocation` _output_1 (`local.L_EvenNumber`)) _relativelocation)))
    (bind (_returnvalue_x_4 _returnvalue_y_2 _returnvalue_z_2) (`KismetMathLibrary.BreakVector` (- (`self.GetLocalLocation` _output_2 (not (`local.L_EvenNumber`))) _relativelocation)))
    (`SplineMeshComponent.SetStartAndEnd` (`local.L_SelectIndexElement`) (`KismetMathLibrary.MakeVector` _returnvalue_x _returnvalue_y _returnvalue_z) (`SplineMeshComponent.GetStartTangent` _l_selectindexelement) (`KismetMathLibrary.MakeVector` _returnvalue_x_2 _returnvalue_y_2 _returnvalue_z_2) (`SplineMeshComponent.GetEndTangent` _l_selectindexelement) true)))

(fn `EndOverlap`
  (params (OverlappedComponent :type "PrimitiveComponent Object Reference") (OtherActor :type "Actor Object Reference") (OtherComp :type "PrimitiveComponent Object Reference") (OtherBodyIndex :type Integer))
  (if (`self.ActorHasTag` OtherActor "GG")
    (`self.SetActorTickEnabled` false)
    (`self.EnableTimer`)
    (return)))

(fn `GenerateConstrain`
  (bind _stm_planks (`self.STM_Planks`))
  (for _index (range (`self.Len`))
    (bind _returnvalue (`AddComponent|NODE_AddPhysicsConstraintComponent-1` :`RelativeTransform` (`KismetMathLibrary.MakeTransform` (0.0 0.0 0.0) (struct :`Pitch` 180.0 :`Roll` 90.0))))
    (bind _output (`|GetArrayItem` _stm_planks _index))
    (`PhysicsConstraintComponent.SetConstrainedComponents` _returnvalue _output "None" (`|GetArrayItem` _stm_planks (+ _index 1)) "None")
    (`SceneComponent.K2_AttachToComponent` _returnvalue _output "None" "KeepRelative" "KeepRelative" "KeepRelative" true)))

(fn `GenerateInstStmRopeWinding`
  (params (InstanceLocation :type "HierarchicalInstancedStaticMeshComponent Object Reference") (MultiplyUpVector :type "Array of Integer"))
  (bind _returnvalue (`AddComponent|NODE_AddHierarchicalInstancedStaticMeshComponent-1`))
  (for _index (range (+ (`InstancedStaticMeshComponent.GetInstanceCount` InstanceLocation) 1))
    (for _array_element MultiplyUpVector
      (bind _outinstancetransform (`InstancedStaticMeshComponent.GetInstanceTransform` InstanceLocation _index false))
      (`InstancedStaticMeshComponent.AddInstance` _returnvalue (`KismetMathLibrary.MakeTransform` (+ (.location _outinstancetransform) (* (`KismetMathLibrary.GetUpVector` (.rotation _outinstancetransform)) _array_element)) (.rotation _outinstancetransform) (1.5 1.5 1.0)) false))))

(fn `GenerateOverlapCapsule`
  (bind _returnvalue (* (`self.Len`) 12.5))
  (bind _returnvalue_2 (+ _returnvalue 100.0))
  (bind _returnvalue_3 (`AddComponent|NODE_AddCapsuleComponent-0` :`RelativeTransform` (`KismetMathLibrary.MakeTransform` (0.0 0.0 0.0) (struct :`Pitch` 90.0))))
  (`SceneComponent.K2_SetRelativeLocation` _returnvalue_3 (`KismetMathLibrary.MakeVector` _returnvalue) false false)
  (`CapsuleComponent.SetCapsuleHalfHeight` _returnvalue_3 _returnvalue_2 true)
  (`CapsuleComponent.SetCapsuleRadius` _returnvalue_3 (/ _returnvalue_2 2.0) true)
  (add `PrimitiveComponent.OnComponentBeginOverlap` _returnvalue_3 (`|CreateDelegate` :!event `BeginOverlap`))
  (add `PrimitiveComponent.OnComponentEndOverlap` _returnvalue_3 (`|CreateDelegate` :!event `EndOverlap`)))

(fn `GeneratePlanks`
  (for _index (range (+ (`self.Len`) 1))
    (bind _returnvalue (`AddComponent|NODE_AddStaticMeshComponent-0` :`RelativeTransform` (`KismetMathLibrary.MakeTransform` (`KismetMathLibrary.MakeVector` (`KismetMathLibrary.Conv_IntToDouble` (* _index 25))) (`KismetMathLibrary.MakeRotator` 0.0 180.0 (select `bool` (> (mod _index 2) 0) :`false` 90.0 :`true` 270.0 :!type "Float (single-precision)")))))
    (`KismetArrayLibrary.Array_Add` (`self.STM_Planks`) _returnvalue))
  (`PrimitiveComponent.SetSimulatePhysics` (`|GetArrayItem` (`self.STM_Planks`)) false)
  (`PrimitiveComponent.SetSimulatePhysics` (`|GetArrayItem` (`self.STM_Planks`) (`KismetArrayLibrary.Array_LastIndex` (`self.STM_Planks`))) false))

(fn `GenerateSplineAtInstSTM`
  (params (Instance :type "HierarchicalInstancedStaticMeshComponent Object Reference") (MultiplyUpVector :type Integer))
  (`|ExecutionSequence`
    (:`then_0`
      _)
    (:`then_1`
      _))
  (bind _isa (`/Engine/EditorBlueprintResources/StandardMacros.FlipFlop`)
    (:`A`
      _)
    (:`B`
      _))
  (bind _returnvalue (`AddComponent|NODE_AddSplineMeshComponent-5`))
  (bind _outinstancetransform (`InstancedStaticMeshComponent.GetInstanceTransform` Instance (select `bool` _isa :`false` 1) false))
  (bind _returnvalue_2 (`KismetMathLibrary.GetForwardVector` (`SceneComponent.RelativeRotation` _returnvalue)))
  (bind _outinstancetransform_2 (`InstancedStaticMeshComponent.GetInstanceTransform` Instance (select `bool` _isa :`false` 3 :`true` 2) false))
  (`SplineMeshComponent.SetStartAndEnd` _returnvalue (+ (.location _outinstancetransform) (* (`KismetMathLibrary.GetUpVector` (.rotation _outinstancetransform)) MultiplyUpVector)) (+ (* _returnvalue_2 500) (0.0 0.0 -100.0)) (+ (.location _outinstancetransform_2) (* (`KismetMathLibrary.GetUpVector` (.rotation _outinstancetransform_2)) MultiplyUpVector)) (+ (* _returnvalue_2 500) (0.0 0.0 100.0)) true))

(fn `Spline`
  (locals (KeySplinePoint :type "Array of SplinePoint Structure"))
  (for (_array_element _array_index) (`self.STM_Planks`)
    (`|ExecutionSequence`
      (:`then_0`
        _)
      (:`then_1`
        _))
    (bind _isa (`/Engine/EditorBlueprintResources/StandardMacros.FlipFlop`)
      (:`A`
        _)
      (:`B`
        _))
    (bind (_relativelocation_x _relativelocation_y _relativelocation_z) (`KismetMathLibrary.BreakVector` (`SceneComponent.RelativeLocation` _array_element)))
    (bind _returnvalue (`AddComponent|NODE_AddSplineMeshComponent-1` :`RelativeTransform` (`KismetMathLibrary.MakeTransform` (`KismetMathLibrary.MakeVector` (+ _relativelocation_x 12.5) _relativelocation_y _relativelocation_z))))
    (bind _returnvalue_2 (select `bool` _isa :`false` (* 55.0 -1.0) :`true` 55.0))
    (`SplineMeshComponent.SetStartAndEnd` _returnvalue (`KismetMathLibrary.MakeVector` (* 12.5 -1.0) _returnvalue_2 -5.0) (-12.5 0.0 0.0) (`KismetMathLibrary.MakeVector` 12.5 _returnvalue_2 -5.0) (12.5 0.0 0.0) true)
    (bind _output (`|GetArrayItem` (`self.STM_Planks`) (+ _array_index 1)))
    (`BlueprintMapLibrary.Map_Add` (`self.NewVar`) _returnvalue (make `/Game/GamePlay_BP/Interacts/RopeBridge/BST_MeshAtSpline` _array_element (select `bool` (`KismetSystemLibrary.IsValid` _output) :`false` _array_element :`true` _output)))))

(fn `UserConstructionScript`
  (bind _returnvalue (/ (* (`self.Len`) 25) 2))
  (if (`self.DebugVisual`)
    (`SceneComponent.K2_SetRelativeTransform` (`self.Cube`) (`KismetMathLibrary.MakeTransform` (`KismetMathLibrary.MakeVector` (`KismetMathLibrary.Conv_IntToDouble` _returnvalue)) (struct) (`KismetMathLibrary.MakeVector` (`KismetMathLibrary.Conv_IntToDouble` (/ _returnvalue 45)) 1.5 0.1)) false false)
    (else
      (`self.GeneratePlanks`)
      (`self.GenerateConstrain`)
      (`self.Spline`)
      (`self.DynamicUpdateSpline`)
      (`self.GenerateOverlapCapsule`)
      (`self.AddInstanceSTM`)
      (`ActorComponent.K2_DestroyComponent` (`self.Cube`)))))