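; BP_Pitfall is a resizable hazard that sends a damage message to actors tagged "GG" when they overlap its box trigger.
; The construction script resets actor scale, sizes the box from InBoxExtent and raises it by its half-height.
; SpawnInstance then rebuilds a grid of hierarchical instanced meshes across the box footprint, with density set by division variables and randomized rotation and XY scale.
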(event `self.Box.OnComponentBeginOverlap`
  (params (OverlappedComponent :type "PrimitiveComponent Object Reference") (OtherActor :type "Actor Object Reference") (OtherComp :type "PrimitiveComponent Object Reference") (OtherBodyIndex :type Integer) (bFromSweep :type Boolean) (SweepResult :type "HitResult Structure (by ref)"))
  (if (`self.ActorHasTag` OtherActor "GG")
    (message `/Game/GamePlay_BP/Interface/BPI_Damage.Damage` OtherActor self 100.0 (0.0 0.0 0.0))))

(fn `SpawnInstance`
  (locals (L_LastIndex_X :type Integer) (L_LastIndex_Y :type Integer) (L_X_Location :type "Float (double-precision)" :default 0.0) (L_Y_Location :type "Float (double-precision)" :default 0.0))
  (bind _in_box_extent_x (`KismetMathLibrary.BreakVector` (`self.In Box Extent`)))
  (bind (_in_box_extent_x_2 _in_box_extent_y) (`KismetMathLibrary.BreakVector` (`self.In Box Extent`)))
  (bind _rotationaddrandom (`self.RotationAddRandom`))
  (bind _rotationaddrandom_2 (`self.RotationAddRandom`))
  (bind _instancescalex (`self.InstanceScaleX`))
  (bind _instancescaley (`self.InstanceScaleY`))
  (bind _addrandomscale (`self.AddRandomScale`))
  (bind (_in_box_extent_x_3 _in_box_extent_y_2 _in_box_extent_z) (`KismetMathLibrary.BreakVector` (`self.In Box Extent`)))
  (bind (_in_box_extent_x_4 _in_box_extent_y_3 _in_box_extent_z_2) (`KismetMathLibrary.BreakVector` (`self.In Box Extent`)))
  (bind _in_box_extent_x_5 (`KismetMathLibrary.BreakVector` (`self.In Box Extent`)))
  (bind (_in_box_extent_x_6 _in_box_extent_y_4) (`KismetMathLibrary.BreakVector` (`self.In Box Extent`)))
  (`|ExecutionSequence`
    (:`then_0`
      (`SceneComponent.K2_SetRelativeLocation` (`self.Box`) (`KismetMathLibrary.MakeVector` 0.0 0.0 _in_box_extent_z) false true))
    (:`then_1`
      (`StaticMeshComponent.SetStaticMesh` (`self.HierarchicalInstancedStaticMesh`) (`self.STM`)))
    (:`then_2`
      (`InstancedStaticMeshComponent.ClearInstances` (`self.HierarchicalInstancedStaticMesh`))
      (bind _output_get (set `local.L_LastIndex_X` (/ (`KismetMathLibrary.FTrunc` _in_box_extent_x) (`self.X_Division`))))
      (for _index (range (+ _output_get 1))
        (set `local.L_X_Location` (`KismetMathLibrary.Lerp` (* _in_box_extent_x_5 -1.0) _in_box_extent_x_5 (/ (`KismetMathLibrary.Conv_IntToDouble` _index) (`KismetMathLibrary.Conv_IntToDouble` (`local.L_LastIndex_X`)))))
        (bind _output_get_2 (set `local.L_LastIndex_Y` (/ (`KismetMathLibrary.FTrunc` _in_box_extent_y_4) (`self.Y_Division`))))
        (for _index_2 (range (+ _output_get_2 1))
          (set `local.L_Y_Location` (`KismetMathLibrary.Lerp` (* _in_box_extent_y -1.0) _in_box_extent_y (/ (`KismetMathLibrary.Conv_IntToDouble` _index_2) (`KismetMathLibrary.Conv_IntToDouble` (`local.L_LastIndex_Y`)))))
          (`InstancedStaticMeshComponent.AddInstance` (`self.HierarchicalInstancedStaticMesh`) (`KismetMathLibrary.MakeTransform` (`KismetMathLibrary.MakeVector` (`local.L_X_Location`) (`local.L_Y_Location`) (+ _in_box_extent_z_2 (`self.AddLocationZ`))) (`KismetMathLibrary.MakeRotator` (`KismetMathLibrary.RandomFloatInRange` (* _rotationaddrandom -1.0) _rotationaddrandom) (`KismetMathLibrary.RandomFloatInRange` (* _rotationaddrandom_2 -1.0) _rotationaddrandom_2) (`KismetMathLibrary.RandomFloatInRange` -180.0 180.0)) (`KismetMathLibrary.MakeVector` (`KismetMathLibrary.RandomFloatInRange` (- _instancescalex _addrandomscale) (+ _instancescalex _addrandomscale)) (`KismetMathLibrary.RandomFloatInRange` (- _instancescaley _addrandomscale) (+ _instancescaley _addrandomscale)) (`self.ScaleZ`))) false))))))

(fn `UserConstructionScript`
  (`self.SetActorScale3D` (1.0 1.0 1.0))
  (`BoxComponent.SetBoxExtent` (`self.Box`) (`self.In Box Extent`) false)
  (`self.SpawnInstance`))