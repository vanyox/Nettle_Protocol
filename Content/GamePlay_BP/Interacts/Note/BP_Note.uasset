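; BP_Note is an interactable note that shows its text on screen in a W_Note widget.
; Overlapping its StartInteractCube toggles the interact trace message on the overlapping actor.
; Interact sets BlockOverlap, creates the widget with InText, binds its destroy event and adds it to the viewport.
; CanInteract refuses further use while BlockOverlap is set, and DestroyWidget clears the flag.
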(event `self.StartInteractCube.OnComponentBeginOverlap`
  (params (OverlappedComponent :type "PrimitiveComponent Object Reference") (OtherActor :type "Actor Object Reference") (OtherComp :type "PrimitiveComponent Object Reference") (OtherBodyIndex :type Integer) (bFromSweep :type Boolean) (SweepResult :type "HitResult Structure (by ref)"))
  (message `/Game/GamePlay_BP/Interface/BPI_CharSetting.UpdateTraceInteract` OtherActor true))

(event `self.StartInteractCube.OnComponentEndOverlap`
  (params (OverlappedComponent :type "PrimitiveComponent Object Reference") (OtherActor :type "Actor Object Reference") (OtherComp :type "PrimitiveComponent Object Reference") (OtherBodyIndex :type Integer))
  (message `/Game/GamePlay_BP/Interface/BPI_CharSetting.UpdateTraceInteract` OtherActor false))

(fn `CanInteract`
  (returns (Return :type Boolean))
  (return (not (`self.BlockOverlap`))))

(fn `DestroyWidget`
  (set `self.BlockOverlap` false))

(fn `Interact`
  (returns (Return :type Boolean))
  (set `self.BlockOverlap` true)
  (bind _returnvalue (`|CreateWidget` "/Game/GamePlay_BP/Interacts/Note/W_Note.W_Note_C" null (`self.In Text`)))
  (add `/Game/GamePlay_BP/Interacts/Note/W_Note.DestroyWidget` _returnvalue (`|CreateDelegate` :!event `DestroyWidget`))
  (`UserWidget.AddToViewport` _returnvalue 1)
  (return true))

(fn `UserConstructionScript`
  (`parent.UserConstructionScript`))