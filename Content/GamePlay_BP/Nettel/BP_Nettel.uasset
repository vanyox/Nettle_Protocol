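; Nettle patch hazard that repeatedly damages a "GG"-tagged actor inside its box, ignoring components tagged "Weapon", via a looping timer.
; The construction script sizes the box and derives Experience from its extent.
; Damage drains Hp; death reports Experience, disables the box and squashes the instanced meshes.
; SpawnInstance randomly scatters mesh instances within the box, but its construction-script call is disconnected.
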(event `self.Box.OnComponentBeginOverlap`
  (params (OverlappedComponent :type "PrimitiveComponent Object Reference") (OtherActor :type "Actor Object Reference") (OtherComp :type "PrimitiveComponent Object Reference") (OtherBodyIndex :type Integer) (bFromSweep :type Boolean) (SweepResult :type "HitResult Structure (by ref)"))
  (`self.HasTag` OtherActor OtherComp)
  (`self.OverlapActor`
    (:`then`)
    (:`else`
      (set `self.OverlapActor` OtherActor)
      (`self.DamageOverlap`))))

(event `self.Box.OnComponentEndOverlap`
  (params (OverlappedComponent :type "PrimitiveComponent Object Reference") (OtherActor :type "Actor Object Reference") (OtherComp :type "PrimitiveComponent Object Reference") (OtherBodyIndex :type Integer))
  (`self.HasTag` OtherActor OtherComp)
  (set `self.OverlapActor` null))

(fn `Damage`
  (params (Init :type "Actor Object Reference") (Damage :type "Float (double-precision)"))
  (returns (Hit :type Boolean))
  (locals (L_NewHp :type "Float (double-precision)"))
  (if (> (`self.Hp`) 0.0)
    (bind _output_get (set `local.L_NewHp` (- (`self.Hp`) (`local.Damage`))))
    (bind _returnvalue (> _output_get 5.0))
    (set `self.B_Dead` (not _returnvalue))
    (set `self.Hp` (select `bool` _returnvalue :`true` (`local.L_NewHp`)))
    (`|ExecutionSequence`
      (:`then_0`
        (if (`self.B_Dead`)
          (`self.F_Dead`)))
      (:`then_1`
        (return true)))
    (else
      (return false))))

(fn `DamageOverlap`
  (`self.OverlapActor`
    (:`then`
      (message `/Game/GamePlay_BP/Interface/BPI_Damage.Damage` (`self.OverlapActor`) self 15.0)
      (if (not (`KismetSystemLibrary.K2_IsTimerActive` null "DamageOverlap"))
        (`KismetSystemLibrary.K2_SetTimer` null "DamageOverlap" 0.5 true)))
    (:`else`
      (`KismetSystemLibrary.K2_ClearTimer` null "DamageOverlap"))))

(fn `F_Dead`
  (bind (_relativelocation_x _relativelocation_y _relativelocation_z) (`KismetMathLibrary.BreakVector` (`SceneComponent.RelativeLocation` (`self.InstancedStaticMesh`))))
  (`self.DDestroy` self (`self.Experience`))
  (`PrimitiveComponent.SetCollisionEnabled` (`self.Box`) "NoCollision")
  (`SceneComponent.SetHiddenInGame` (`self.Box`) true false)
  (for _index (range (`InstancedStaticMeshComponent.GetInstanceCount` (`self.InstancedStaticMesh`)))
    (bind _outinstancetransform (`InstancedStaticMeshComponent.GetInstanceTransform` (`self.InstancedStaticMesh`) _index false))
    (`InstancedStaticMeshComponent.UpdateInstanceTransform` (`self.InstancedStaticMesh`) _index (`KismetMathLibrary.MakeTransform` (`KismetMathLibrary.MakeVector` (.x (.location _outinstancetransform)) (.y (.location _outinstancetransform)) (* _relativelocation_z -1.0)) (.rotation _outinstancetransform) (`KismetMathLibrary.MakeVector` (.x (.scale _outinstancetransform)) (.y (.scale _outinstancetransform)) 0.1)) false true false)))

(fn `SpawnInstance`
  (locals (L_max :type Integer) (L_ZRandom :type "Float (double-precision)" :default 0.0))
  (bind (_boxextent_x _boxextent_y) (`KismetMathLibrary.BreakVector` (`BoxComponent.BoxExtent` (`self.Box`))))
  (bind (_boxextent_x_2 _boxextent_y_2) (`KismetMathLibrary.BreakVector` (`BoxComponent.BoxExtent` (`self.Box`))))
  (bind _returnvalue (- _boxextent_y_2 5.0))
  (bind _returnvalue_2 (- _boxextent_x_2 5.0))
  (`InstancedStaticMeshComponent.ClearInstances` (`self.InstancedStaticMesh`))
  (set `local.L_max` (`KismetMathLibrary.RandomIntegerInRange` 5 (`KismetMathLibrary.FTrunc` (/ (+ _boxextent_x _boxextent_y) 5.0))))
  (for _ (range (+ (`local.L_max`) 1))
    (set `local.L_ZRandom` (`KismetMathLibrary.RandomFloatInRange` 0.5 1.5))
    (`InstancedStaticMeshComponent.AddInstance` (`self.InstancedStaticMesh`) (`KismetMathLibrary.MakeTransform` (`KismetMathLibrary.MakeVector` (`KismetMathLibrary.RandomFloatInRange` (* _returnvalue_2 -1.0) _returnvalue_2) (`KismetMathLibrary.RandomFloatInRange` (* _returnvalue -1.0) _returnvalue) (`KismetMathLibrary.MapRangeClamped` (`local.L_ZRandom`) 0.5 1.5 -25.0 25.0)) (struct) (`KismetMathLibrary.MakeVector` 0.07 0.07 (`local.L_ZRandom`))) false)))

(fn `UserConstructionScript`
  (locals (L_max :type Integer))
  (bind (_in_box_extent_x _in_box_extent_y _in_box_extent_z) (`KismetMathLibrary.BreakVector` (`self.In Box Extent`)))
  (`self.SetActorScale3D` (1.0 1.0 1.0))
  (`|ExecutionSequence`
    (:`then_0`
      (if (not (or (< _in_box_extent_x 1.0) (< _in_box_extent_y 1.0) (< _in_box_extent_z 1.0)))
        (`BoxComponent.SetBoxExtent` (`self.Box`) (`self.In Box Extent`) false)))
    (:`then_1`
      (set `self.Experience` (`KismetMathLibrary.VSize` (`BoxComponent.BoxExtent` (`self.Box`)))))))