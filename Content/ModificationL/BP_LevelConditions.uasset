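; BP_LevelConditions is a level setup actor that trims the nettle actors and passes level settings to the HUD.
; On BeginPlay, it randomly destroys nettles down to a nonzero cap, sparing those tagged AlwaysSpawn, then hides the rest and disables their collision.
; It then sends the nettle list, start time and three experience values to B_HUD.
; The construction script records the total nettle count.
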(event `self.ReceiveBeginPlay`
  (`self.FilterNettle`)
  (bind _asb_hud (cast `/Game/GamePlay_BP/Base/B_HUD` (`PlayerController.GetHUD` (`GameplayStatics.GetPlayerController` 0))))
  (`/Game/GamePlay_BP/Base/B_HUD.UpdateInfoNettle` _asb_hud (`self.Nettles`))
  (`/Game/GamePlay_BP/Base/B_HUD.InitTime` _asb_hud (`KismetMathLibrary.Conv_IntToDouble` (`self.StartTime`)))
  (`/Game/GamePlay_BP/Base/B_HUD.NewExp` _asb_hud (`|MakeArray` (`KismetMathLibrary.Conv_IntToDouble` (`self.Small`)) (`KismetMathLibrary.Conv_IntToDouble` (`self.Medium`)) (`KismetMathLibrary.Conv_IntToDouble` (`self.Big`)))))

(fn `FilterNettle`
  (locals (L_SelIndexDell :type "Actor Object Reference"))
  (`|ExecutionSequence`
    (:`then_0`
      (if (!= (`self.MaxNettleInLevel`) 0)
        (if (not (<= (`KismetArrayLibrary.Array_Length` (`self.Nettles`)) (`self.MaxNettleInLevel`))) :!label _label
          (set `local.L_SelIndexDell` (`KismetArrayLibrary.Array_Random` (`self.Nettles`)))
          (if (not (`self.ActorHasTag` (`local.L_SelIndexDell`) "AlwaysSpawn"))
            (`self.K2_DestroyActor` (`local.L_SelIndexDell`))
            (`KismetArrayLibrary.Array_RemoveItem` (`self.Nettles`) (`local.L_SelIndexDell`))
            (goto _label)
            (else
              (goto _label))))))
    (:`then_1`
      (for _array_element (`self.Nettles`)
        (`self.SetActorHiddenInGame` _array_element true)
        (`self.SetActorEnableCollision` _array_element false)))))

(fn `UpdateLenNettle`
  (set `self.TotalNettlesAtTheLevel` (`KismetArrayLibrary.Array_Length` (`self.Nettles`))))

(fn `UserConstructionScript`
  (`self.UpdateLenNettle`))