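; BP_MW_Wind is a placeable wind controller actor that feeds global wind settings to materials through the MPC_MW_Controller parameter collection.
; It writes its Intensity and Speed variables as scalar parameters and its root component's forward vector as the wind direction, so rotating the actor aims the wind.
; The construction script applies the values in the editor, and Tick rewrites the same values every frame at runtime.
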(event `self.ReceiveTick`
  (params (DeltaSeconds :type "Float (single-precision)"))
  (`KismetMaterialLibrary.SetScalarParameterValue` "/Game/MWCommon/_Legacy/Materials/MASTER/Par/MPC_MW_Controller.MPC_MW_Controller" "MW_WindIntensity" (`self.Intensity`))
  (`KismetMaterialLibrary.SetScalarParameterValue` "/Game/MWCommon/_Legacy/Materials/MASTER/Par/MPC_MW_Controller.MPC_MW_Controller" "MW_WindSpeed" (`self.Speed`))
  (`KismetMaterialLibrary.SetVectorParameterValue` "/Game/MWCommon/_Legacy/Materials/MASTER/Par/MPC_MW_Controller.MPC_MW_Controller" "MW_WindDirection" (`KismetMathLibrary.Conv_VectorToLinearColor` (`SceneComponent.GetForwardVector` (`self.DefaultSceneRoot`)))))

(fn `UserConstructionScript`
  (`KismetMaterialLibrary.SetScalarParameterValue` "/Game/MWCommon/_Legacy/Materials/MASTER/Par/MPC_MW_Controller.MPC_MW_Controller" "MW_WindIntensity" (`self.Intensity`))
  (`KismetMaterialLibrary.SetScalarParameterValue` "/Game/MWCommon/_Legacy/Materials/MASTER/Par/MPC_MW_Controller.MPC_MW_Controller" "MW_WindSpeed" (`self.Speed`))
  (`KismetMaterialLibrary.SetVectorParameterValue` "/Game/MWCommon/_Legacy/Materials/MASTER/Par/MPC_MW_Controller.MPC_MW_Controller" "MW_WindDirection" (`KismetMathLibrary.Conv_VectorToLinearColor` (`SceneComponent.GetForwardVector` (`self.DefaultSceneRoot`)))))