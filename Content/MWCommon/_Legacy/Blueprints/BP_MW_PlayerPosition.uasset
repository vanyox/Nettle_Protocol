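; Legacy helper Blueprint that feeds player position and movement into the MPC_MW_Controller material parameter collection every tick.
; It writes the pawn's location and its clamped, unsmoothed speed for materials to read.
; It also writes an interpolated bend position trailing behind the pawn's forward vector, with the offset scaled by speed.
; A smoothed, normalized PlayerSpeed is stored but not sent to the collection.
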(event `self.ReceiveTick`
  (params (DeltaSeconds :type "Float (single-precision)"))
  (bind _returnvalue (`GameplayStatics.GetWorldDeltaSeconds`))
  (bind _returnvalue_2 (`GameplayStatics.GetPlayerPawn` (`self.PlayerPawnIndex`)))
  (bind _returnvalue_3 (`self.K2_GetActorLocation` _returnvalue_2))
  (bind _returnvalue_4 (`KismetMathLibrary.FClamp` (`KismetMathLibrary.VSize` (`self.GetVelocity` _returnvalue_2)) 0.0 400.0))
  (bind _returnvalue_5 (`KismetMathLibrary.VInterpTo` (`self.BendPos`) (+ _returnvalue_3 (* (`KismetMathLibrary.NegateVector` (`self.GetActorForwardVector` _returnvalue_2)) (* (`self.BendPosLength`) _returnvalue_4))) _returnvalue 10.0))
  ;[1 1 1] PlayerPosition
  (`KismetMaterialLibrary.SetVectorParameterValue` "/Game/MWCommon/_Legacy/Materials/MASTER/Par/MPC_MW_Controller.MPC_MW_Controller" "MW_PlayerPosition" (`KismetMathLibrary.Conv_VectorToLinearColor` _returnvalue_3))
  ;[1 1 1] PlayerSpeed
  (set `self.PlayerSpeed` (`KismetMathLibrary.FInterpTo` (`self.PlayerSpeed`) (/ _returnvalue_4 400.0) _returnvalue 5.0))
  (`KismetMaterialLibrary.SetScalarParameterValue` "/Game/MWCommon/_Legacy/Materials/MASTER/Par/MPC_MW_Controller.MPC_MW_Controller" "MW_PlayerSpeed" _returnvalue_4)
  ;[1 1 1] PayerBendPosition
  (set `self.BendPos` _returnvalue_5)
  (`KismetMaterialLibrary.SetVectorParameterValue` "/Game/MWCommon/_Legacy/Materials/MASTER/Par/MPC_MW_Controller.MPC_MW_Controller" "MW_BendPos" (`KismetMathLibrary.Conv_VectorToLinearColor` _returnvalue_5)))

(fn `UserConstructionScript`)